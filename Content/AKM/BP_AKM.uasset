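; AKM weapon Blueprint that gives the player automatic hitscan fire with magazine and reserve ammo.
; Left mouse runs ShootFunc on a looping timer, playing a montage, spending ammo and debug-drawing an offset camera line trace.
; Any blocking hit sets the player controller's Health to a fixed value.
; ReloadFunc instantly refills from reserve on input or when Tick finds the magazine empty; releasing T runs a socket attachment on the player mesh.
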(event `Key|T`
  (params (Key :type "Key Structure"))
  (bind _returnvalue (`GameplayStatics.GetPlayerCharacter` 0))
  ;[1 1 1] Spawn
  (:`Released`
    (`self.K2_AttachToComponent` _returnvalue (`Character.Mesh` _returnvalue) "Sockettt" "SnapToTarget" "KeepRelative" "KeepRelative" false)))

(event `self.ReceiveBeginPlay`
  ;[1 1 1] Enable Input
  (`self.EnableInput` (`GameplayStatics.GetPlayerController` 0)))

(event `InputAction|Reload`
  (params (Key :type "Key Structure"))
  ;[1 1 1] Reload Mechanic
  (:`Pressed`
    (`self.ReloadFunc`)))

(event `Key|LeftMouseButton`
  (params (Key :type "Key Structure"))
  ;[1 1 1] Shooting Mechanic
  (:`Pressed`
    (`|ExecutionSequence`
      (:`then_0`
        (`self.ShootFunc`))
      (:`then_1`
        (`KismetSystemLibrary.K2_SetTimer` null "ShootFunc" 0.15 true))))
  (:`Released`
    (`KismetSystemLibrary.K2_ClearTimer` null "ShootFunc")))

(event `self.ReceiveTick`
  (params (DeltaSeconds :type "Float (single-precision)"))
  ;[1 1 1] Reload Mechanic
  (if (<= (`self.CurrentAmmo`) 0)
    (`self.ReloadFunc`)))

(fn `ReloadFunc`
  (while (and (<= (`self.CurrentAmmo`) 29) (>= (`self.Ammo`) 1))
    (`/Engine/EditorBlueprintResources/StandardMacros.IncrementInt` (`self.CurrentAmmo`)
      (:`  `
        (`/Engine/EditorBlueprintResources/StandardMacros.DecrementInt` (`self.Ammo`))))))

(fn `ShootFunc`
  (if (not (<= (`self.CurrentAmmo`) 0))
    (bind _asfirst_person_character (cast `/Game/FirstPersonBP/Blueprints/FirstPersonCharacter` (`GameplayStatics.GetPlayerCharacter` 0)))
    (`AnimInstance.Montage_Play` (`SkeletalMeshComponent.GetAnimInstance` (`/Game/FirstPersonBP/Blueprints/FirstPersonCharacter.Mesh2P` _asfirst_person_character)) "/Game/FirstPerson/Animations/FirstPersonFire_Montage.FirstPersonFire_Montage" 1.0 "MontageLength" 0.0)
    (bind _asfirst_person_character_2 (cast `/Game/FirstPersonBP/Blueprints/FirstPersonCharacter` (`GameplayStatics.GetPlayerCharacter` 0)))
    (`/Engine/EditorBlueprintResources/StandardMacros.DecrementInt` (`self.CurrentAmmo`)
      (:`  `
        (bind _firstpersoncamera (`/Game/FirstPersonBP/Blueprints/FirstPersonCharacter.FirstPersonCamera` _asfirst_person_character_2))
        (bind _returnvalue (`SceneComponent.K2_GetComponentLocation` _firstpersoncamera))
        (bind _outhit (`KismetSystemLibrary.LineTraceSingle` :`Start` (`KismetMathLibrary.MakeVector` (.x _returnvalue) (.y _returnvalue) (.z _returnvalue)) :`End` (+ _returnvalue (* (`KismetMathLibrary.GetForwardVector` (`KismetMathLibrary.MakeRotator` (.roll (`SceneComponent.K2_GetComponentRotation` _firstpersoncamera)) (- (.pitch (`SceneComponent.K2_GetComponentRotation` _firstpersoncamera)) 3.0) (+ (.yaw (`SceneComponent.K2_GetComponentRotation` _firstpersoncamera)) 0.7))) 1500.0)) :`TraceChannel` "TraceTypeQuery1" :`bTraceComplex` true :`DrawDebugType` "ForDuration"))
        (bind _asplayer_controller_bp (cast `/Game/FirstPersonBP/Blueprints/PlayerControllerBP` (`GameplayStatics.GetPlayerController` 0)))
        (if (`GameplayStatics.BreakHitResult` _outhit)
          (set `/Game/FirstPersonBP/Blueprints/PlayerControllerBP.Health` 22 _asplayer_controller_bp))))))

(fn `UserConstructionScript`)